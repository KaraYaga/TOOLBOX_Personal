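; Base dialogue component that runs branching conversations through a WBP_Dialogue widget it creates and removes.
; Each progression resets the index and calls the empty Dialogue function, presumably overridden by children to chain AddDialogue calls.
; AddDialogue returns stored choices for completed steps or displays an unanswered one, so the tree replays after every selection.
; Progress can be cleared or stepped back, and changing the tree index clears it.
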(fn `AddDialogue`
  (params (Speaker :type Text) (Dialogue :type Text) (OptionsText :type "Array of Text"))
  (returns (State :type "/Game/TOOLBOX/Dialogue_Tool/BluePrints/ENUM_DialogueState Enum") (OptionIndex :type Integer))
  (bind (_value _returnvalue) (`BlueprintMapLibrary.Map_Find` (`self.DialogueProgress`) (`self.DialogueIndex`)))
  ;[1 1 1] Add Next Dialogue Option (++ Index)
  (`/Engine/EditorBlueprintResources/StandardMacros.IncrementInt` (`self.DialogueIndex`) ; Increment Dialogue Index Value, \nDialogue Index starts at -1 \nso your first Dialogue addition will =0
    (:`  `
      (if _returnvalue
        (return "NewEnumerator0" _value) ; Dialogue had already been Done
        (else
          (`/Game/TOOLBOX/Dialogue_Tool/Widgets/WBP_Dialogue.UpdateDialogueText` (`self.DialogueWidget`) (`self.DialogueIndex`) Speaker Dialogue OptionsText) ; Update the Dialogue,\nAdd it to the Add
          (return "NewEnumerator1" 0) ; Dialogue had already been Done
        )))))

(fn `ClearDialogueProgress`
  ;[1 1 1] Clear Options
  (`BlueprintMapLibrary.Map_Clear` (`self.DialogueProgress`)))

(fn `CloseConversation`
  ;[1 1 1] Close Conversation
  (`Widget.RemoveFromParent` (`self.DialogueWidget`)) ; Close/Remove Widget
)

(fn `Dialogue`)

(fn `OpenConversation`
  ;[1 1 1] Open Conversation
  (bind _returnvalue (`|CreateWidget` "/Game/TOOLBOX/Dialogue_Tool/Widgets/WBP_Dialogue.WBP_Dialogue_C" null self)) ; Access Dialogue Widget
  (bind _output_get (set `self.DialogueWidget` _returnvalue))
  (`UserWidget.AddToViewport` _output_get 0) ; Add to Viewport
  (`self.ProgressDialogue`) ; Next Function
)

(fn `ProgressDialogue`
  ;[1 1 1] Progress Dialogue, Reset Index, Check Tree Index
  (set `self.DialogueIndex` -1) ; Reset Dialogue Index
  (`self.Dialogue`) ; Choose Next Dialogue
)

(fn `RemoveDialogueProfress`
  (params (ProgressSteps :type Integer))
  ;[1 1 1] Remove (Go Back in Index)
  (for _index (range (+ ProgressSteps 1))
    (`BlueprintMapLibrary.Map_Remove` (`self.DialogueProgress`) (- (`self.DialogueIndex`) _index)) ; Remove from Option
  ))

(fn `SetDialogueTreeIndex`
  (params (DialgoueTreeIndex :type Integer))
  ;[1 1 1] Clear Previous Index
  (set `self.DialogueTreeIndex` DialgoueTreeIndex)
  (`self.ClearDialogueProgress`) ; Clear Previous Index
)

(fn `UpdateSelectedOption`
  (params (ProgressIndex :type "Integer (by ref)") (OptionIndex :type "Integer (by ref)"))
  ;[1 1 1] Check Option, UPDATE, Progress
  (`BlueprintMapLibrary.Map_Add` (`self.DialogueProgress`) ProgressIndex OptionIndex)
  (`self.ProgressDialogue`) ; Progress Dialogue Tree
)