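; BP_Shrinker is an actor whose Sphere component shrinks when something overlaps its Collider and grows back when the overlap ends.
; Overlap events ignore actors tagged "Shrinker", then play or reverse a Timeline that lerps the sphere's world scale between BigSize and SmallSize.
; Duration sets the Timeline play rate, and the construction script sizes the Collider from DetectionRadius.
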(event `self.Collider.OnComponentBeginOverlap`
  (params (OverlappedComponent :type "PrimitiveComponent Object Reference") (OtherActor :type "Actor Object Reference") (OtherComp :type "PrimitiveComponent Object Reference") (OtherBodyIndex :type Integer) (bFromSweep :type Boolean) (SweepResult :type "HitResult Structure (by ref)"))
  ;[0.04167 0.04167 0.04167] Shrink/Grow
  (if (not (`self.ActorHasTag` OtherActor "Shrinker"))
    (`self.SetActorRelativeScale3D` (`self.BigSize`))
    (`TimelineComponent.SetPlayRate` (`self.Shrink`) (/ 1.0 (`self.Duration`)))
    (bind (_direction _size) (`Timeline|Shrink` :!label _label) ; Shrinking animation
      (:`Update`
        (`SceneComponent.SetWorldScale3D` (`self.Sphere`) (`KismetMathLibrary.VLerp` (`self.BigSize`) (`self.SmallSize`) _size))))))

(event `self.Collider.OnComponentEndOverlap`
  (params (OverlappedComponent :type "PrimitiveComponent Object Reference") (OtherActor :type "Actor Object Reference") (OtherComp :type "PrimitiveComponent Object Reference") (OtherBodyIndex :type Integer))
  ;[0.04167 0.04167 0.04167] Shrink/Grow
  ;;[0.03646 0.03646 0.03646] Reverse
  (if (not (`self.ActorHasTag` OtherActor "Shrinker"))
    (goto _label :!via `Reverse`)))

(fn `UserConstructionScript`
  (`SphereComponent.SetSphereRadius` (`self.Collider`) (`self.Detection Radius`) true))