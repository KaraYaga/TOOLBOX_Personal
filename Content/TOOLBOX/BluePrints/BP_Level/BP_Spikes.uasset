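; BP_Spikes is a level hazard that destroys player 0's pawn when it overlaps the spikes.
; The construction script builds a configurable width-by-length grid of collision-free cone meshes with a shared material.
; A single Hitbox is centered using the last root child's position and sized from the grid dimensions, handling the kill through its begin-overlap event.
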(event `self.Hitbox.OnComponentBeginOverlap`
  (params (OverlappedComponent :type "PrimitiveComponent Object Reference") (OtherActor :type "Actor Object Reference") (OtherComp :type "PrimitiveComponent Object Reference") (OtherBodyIndex :type Integer) (bFromSweep :type Boolean) (SweepResult :type "HitResult Structure (by ref)"))
  ;[0.4219 0.4219 0.4219] Check if the player collides with the spike
  (if (== OtherActor (`GameplayStatics.GetPlayerPawn` 0))
    (`self.K2_DestroyActor` OtherActor) ; Kill the player
  ))

(fn `UserConstructionScript`
  (bind _children (`SceneComponent.GetChildrenComponents` (`self.DefaultSceneRoot`) false))
  (bind (_relativelocation_x _relativelocation_y _relativelocation_z) (`KismetMathLibrary.BreakVector` (`SceneComponent.RelativeLocation` (`|GetArrayItem` _children (`KismetArrayLibrary.Array_LastIndex` _children)))))
  ;[0.4896 0.4896 0.4896] Places spikes in line
  (for _index (range (+ (`self.spikeLength`) 1))
    (for _index_2 (range (+ (`self.spikeWidth`) 1))
      (bind _returnvalue (`AddComponent|NODE_AddStaticMeshComponent-0` :`RelativeTransform` (`KismetMathLibrary.MakeTransform` (`KismetMathLibrary.MakeVector` (`KismetMathLibrary.Conv_IntToDouble` (* _index_2 50)) (`KismetMathLibrary.Conv_IntToDouble` (* _index 50)) 50.0)))) ; Creates a cone mesh
      (`PrimitiveComponent.SetMaterial` _returnvalue 0 (`self.Material`)) ; Applies material to the created cone
      (`PrimitiveComponent.SetCollisionEnabled` _returnvalue "NoCollision") ; Disables collision on the created cone
    ))
  ;[0.401 0.401 0.401] Places the collider box in the center of the spikes group
  (`SceneComponent.K2_SetRelativeLocation` (`self.Hitbox`) (`KismetMathLibrary.MakeVector` (/ _relativelocation_x 2.0) (/ _relativelocation_y 2.0) _relativelocation_z) false false) ; Set the position of the kill hitbox
  (`BoxComponent.SetBoxExtent` (`self.Hitbox`) (`KismetMathLibrary.MakeVector` (* (+ (`KismetMathLibrary.Conv_IntToDouble` (`self.spikeWidth`)) 1.0) 20.0) (* (+ (`KismetMathLibrary.Conv_IntToDouble` (`self.spikeLength`)) 1.0) 20.0) 32.0) true) ; Set the size of the kill hitbox
)