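; BP_FlashLightSwitchJump is a level actor that briefly flashes one of its two point lights when another actor overlaps it.
; A FlipFlop on the overlap event alternates between PointLight and PointLight1 on successive triggers.
; The chosen light becomes visible, then hides again after a short Delay.
; The overlap is not filtered by actor type, and BeginPlay and the construction script are empty.
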(event `self.ReceiveBeginPlay`)

(event `self.ReceiveActorBeginOverlap`
  (params (OtherActor :type "Actor Object Reference"))
  ;[1 1 1] On Overlap Flip Between Lights
  (`/Engine/EditorBlueprintResources/StandardMacros.FlipFlop` ; Change Light
    (:`A`
      (`SceneComponent.SetVisibility` (`self.PointLight`) true false)
      (`KismetSystemLibrary.Delay` 0.5)
      (`SceneComponent.SetVisibility` (`self.PointLight`) false false))
    (:`B`
      (`SceneComponent.SetVisibility` (`self.PointLight1`) true false)
      (`KismetSystemLibrary.Delay` 0.5)
      (`SceneComponent.SetVisibility` (`self.PointLight1`) false false))))

(fn `UserConstructionScript`)