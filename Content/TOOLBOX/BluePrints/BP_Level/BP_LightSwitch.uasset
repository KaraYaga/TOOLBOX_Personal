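; BP_LightSwitch is a level light switch that toggles a PointLight when the BP_ThirdPersonCharacter overlaps it.
; The construction script sets light visibility and the TurnON label (TurnONText or TurnOFFText) from IsON.
; Each overlap applies the state IsON currently holds, then inverts the flag, so the first overlap repeats the construction state and visible toggling starts with the second.
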(event `self.ReceiveActorBeginOverlap`
  (params (OtherActor :type "Actor Object Reference"))
  (bind _pointlight (`self.PointLight`))
  ;[1 1 1] Turn Light On and Off
  (cast `/Game/ThirdPerson/Blueprints/BP_ThirdPersonCharacter` OtherActor)
  (if (`self.isON`)
    (`SceneComponent.SetVisibility` _pointlight true false) ; IS ON
    (`TextRenderComponent.K2_SetText` (`self.TurnON`) (`self.TurnON Text`))
    (set `self.isON` false)
    (else
      (`SceneComponent.SetVisibility` _pointlight false false) ; IS OFF
      (`TextRenderComponent.K2_SetText` (`self.TurnON`) (`self.TurnOFF text`))
      (set `self.isON` true))))

(fn `UserConstructionScript`
  (bind _pointlight (`self.PointLight`))
  ;[1 1 1] Light Within Level
  (if (`self.isON`)
    (`TextRenderComponent.K2_SetText` (`self.TurnON`) (`self.TurnON Text`))
    (`SceneComponent.SetVisibility` _pointlight true false)
    (else
      (`TextRenderComponent.K2_SetText` (`self.TurnON`) (`self.TurnOFF text`))
      (`SceneComponent.SetVisibility` _pointlight false false))))