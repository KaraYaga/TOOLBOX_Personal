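; BP_Camera is an enemy camera that detects the player through a sphere overlap.
; When the player pawn enters the sphere, it zeroes its RotatingMovement rate and reveals an alert TextRender.
; When the pawn leaves, it restores rotation and hides the alert, printing a debug message on both transitions.
; Detection relies on overlap alone, with no line-of-sight check.
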(event `self.Sphere.OnComponentBeginOverlap`
  (params (OverlappedComponent :type "PrimitiveComponent Object Reference") (OtherActor :type "Actor Object Reference") (OtherComp :type "PrimitiveComponent Object Reference") (OtherBodyIndex :type Integer) (bFromSweep :type Boolean) (SweepResult :type "HitResult Structure (by ref)"))
  ;[1 1 1] On SEEN
  (if (== OtherActor (`GameplayStatics.GetPlayerPawn` 0))
    (`KismetSystemLibrary.PrintString` "I see you") ; Debug SEEN
    (set `RotatingMovementComponent.RotationRate` (struct) (`self.RotatingMovement`))
    (`SceneComponent.SetHiddenInGame` (`self.TextRender`) false false) ; Set ALERT! hidden
  ))

(event `self.Sphere.OnComponentEndOverlap`
  (params (OverlappedComponent :type "PrimitiveComponent Object Reference") (OtherActor :type "Actor Object Reference") (OtherComp :type "PrimitiveComponent Object Reference") (OtherBodyIndex :type Integer))
  ;[1 1 1] On UNSEEN
  (if (== OtherActor (`GameplayStatics.GetPlayerPawn` 0))
    (`KismetSystemLibrary.PrintString` "Where'd they go?") ; Debug UNSEEN
    (set `RotatingMovementComponent.RotationRate` (struct :`Yaw` 180.0) (`self.RotatingMovement`))
    (`SceneComponent.SetHiddenInGame` (`self.TextRender`) true false) ; Hide ALERT!
  ))

(fn `UserConstructionScript`)